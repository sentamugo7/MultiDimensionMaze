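; MazeBuildBP is an actor Blueprint that relays maze-building events to the UI and game state in a multi-dimension maze game.
; Events for win display, fireworks sound, dimension-transition percent and animation finish each look up the first top-level MazeWBP widget and call its matching function.
; DisplayRandSeed instead stores the seed on MultiDimensionMazeGameStateBaseBP.
; The graph holds no maze-generation logic, and its construction script is empty.
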(event EventBeginPlay)

(event Collision|EventActorBeginOverlap
  (params (OtherActor :type Actor%20Object%20Reference)))

(event EventTick
  (params (DeltaSeconds :type Float%20%28single-precision%29)))

(event EventEndShowWin
  (bind _foundwidgets (Widget|GetAllWidgetsOfClass "/Game/Maps/MazeWBP.MazeWBP_C" true))
  (Default|EndShowWin (Utilities|Array|Get(acopy) _foundwidgets)))

(event EventStartShowWin
  (bind _foundwidgets (Widget|GetAllWidgetsOfClass "/Game/Maps/MazeWBP.MazeWBP_C" true))
  (Default|StartShowWin (Utilities|Array|Get(acopy) _foundwidgets)))

(event EventPlayFireworksSound
  (bind _foundwidgets (Widget|GetAllWidgetsOfClass "/Game/Maps/MazeWBP.MazeWBP_C" true))
  (Default|PlayFireworksSound (Utilities|Array|Get(acopy) _foundwidgets)))

(event EventDisplayRandSeed
  (params (randSeed :type Integer))
  (bind _asmulti_dimension_maze_game_state_base_bp (Utilities|Casting|CastToMultiDimensionMazeGameStateBaseBP (Game|GetGameState)))
  (Variables|/Game/Blueprints/MultiDimensionMazeGameStateBaseBP.MultiDimensionMazeGameStateBaseBP_C|SetRandSeed _asmulti_dimension_maze_game_state_base_bp randSeed))

(event EventDisplayDimensionTransition
  (params (displayPercent :type Float%20%28single-precision%29))
  (bind _foundwidgets (Widget|GetAllWidgetsOfClass "/Game/Maps/MazeWBP.MazeWBP_C" true))
  (Default|DisplayDimensionTransition (Utilities|Array|Get(acopy) _foundwidgets) displayPercent))

(event EventFinishAnimation
  (bind _foundwidgets (Widget|GetAllWidgetsOfClass "/Game/Maps/MazeWBP.MazeWBP_C" true))
  (Default|FinishAnimation (Utilities|Array|Get(acopy) _foundwidgets)))

(fn ConstructionScript)